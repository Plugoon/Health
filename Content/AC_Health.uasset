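; Health component that holds a current value, initialised to the maximum on BeginPlay, with getters for both.
; Adding and removing clamp between zero and the maximum, and negative amounts are redirected to the opposite operation.
; Listeners subscribe uniquely and receive OnChange after each adjustment, preceded by OnFull or OnEmpty when a limit is reached.
; A ForeachListener macro shares the loop and validity check across all three notifications.
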(event Custom|CallOnChange
  (params (Value :type Integer))
  ;[1 1 1] Calls
  (bind _outputpin (Utilities|ForeachListener)
    (:Is%20Valid
      (Default|OnChange _outputpin Value))))

(event Custom|CallOnFull
  (params (Value :type Integer))
  ;[1 1 1] Calls
  (bind _outputpin (Utilities|ForeachListener)
    (:Is%20Valid
      (Default|OnFull _outputpin Value))))

(event Custom|CallOnEmpty
  (params (Value :type Integer))
  ;[1 1 1] Calls
  (bind _outputpin (Utilities|ForeachListener)
    (:Is%20Valid
      (Default|OnEmpty _outputpin Value))))

(event Custom|_AddValue
  (params (Value :type Integer))
  (if (>= Value 0)
    (if (< (+ Value (Variables|Plugoon|Health|GetcurrentValue)) (Variables|Plugoon|Health|GetmaxValue))
      (bind _output_get (Variables|Plugoon|Health|SetcurrentValue (+ Value (Variables|Plugoon|Health|GetcurrentValue))))
      (else
        (bind _output_get_2 (Variables|Plugoon|Health|SetcurrentValue (Variables|Plugoon|Health|GetmaxValue)))
        (CallFunction|CallonFull _output_get_2)))
    (CallFunction|CallonChange _output_get)
    (else
      (CallFunction|RemoveValue (* Value -1)))))

(event Custom|_RemoveValue
  (params (Value :type Integer))
  (if (>= Value 0)
    (if (> (- (Variables|Plugoon|Health|GetcurrentValue) Value) 0)
      (bind _output_get (Variables|Plugoon|Health|SetcurrentValue (- (Variables|Plugoon|Health|GetcurrentValue) Value)))
      (else
        (bind _output_get_2 (Variables|Plugoon|Health|SetcurrentValue 0))
        (CallFunction|CallonEmpty _output_get_2)))
    (CallFunction|CallonChange _output_get)
    (else
      (CallFunction|AddValue (* Value -1)))))

(event EventUnsubscribe
  (params (Subscriber :type I%20Health%20Listener%20Interface))
  ;[1 1 1] Subscribe & Unsubscribe
  (Utilities|Array|RemoveItem (Variables|Plugoon|Health|GetHealthListener) Subscriber))

(event EventSubscribe
  (params (Subscribe :type I%20Health%20Listener%20Interface))
  ;[1 1 1] Subscribe & Unsubscribe
  (Utilities|Array|AddUnique (Variables|Plugoon|Health|GetHealthListener) Subscribe))

(event EventAddValue
  (params (Value :type Integer))
  (CallFunction|AddValue Value))

(event EventRemoveValue
  (params (Value :type Integer))
  (CallFunction|RemoveValue Value))

(event EventBeginPlay
  (Variables|Plugoon|Health|SetcurrentValue (Variables|Plugoon|Health|GetmaxValue)))

(fn GetMaxValue
  (return (Variables|Plugoon|Health|GetmaxValue)))

(fn GetValue
  (return (Variables|Plugoon|Health|GetcurrentValue)))